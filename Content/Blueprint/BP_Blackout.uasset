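; Blackout mesh that fades away while the player is inside its box trigger and fades back in when they leave.
; The construction script creates a dynamic instance of MI_Blackout on the mesh and applies the initial Opacity.
; Box overlap events, filtered to BP_Player, call Invisible and Visible, which each play their own timeline to lerp the material's Opacity parameter.
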(event OnComponentBeginOverlap(Box)
  (params (OverlappedComponent :type Primitive%20Component%20Object%20Reference) (OtherActor :type Actor%20Object%20Reference) (OtherComp :type Primitive%20Component%20Object%20Reference) (OtherBodyIndex :type Integer) (bFromSweep :type Boolean) (SweepResult :type Hit%20Result%20Structure%20%28by%20ref%29))
  (Utilities|Casting|CastToBP_Player OtherActor)
  (CallFunction|Invisible))

(event OnComponentEndOverlap(Box)
  (params (OverlappedComponent :type Primitive%20Component%20Object%20Reference) (OtherActor :type Actor%20Object%20Reference) (OtherComp :type Primitive%20Component%20Object%20Reference) (OtherBodyIndex :type Integer))
  (Utilities|Casting|CastToBP_Player OtherActor)
  (CallFunction|Visible))

(event Custom|Invisible
  (bind _alpha (Timeline|TimelineInvisible Play)
    (:Update
      (Variables|Default|SetOpacity (Math|Float|Lerp 1.0 0.0 _alpha))
      (Rendering|Material|SetScalarParameterValue (Variables|Default|GetMaterial) "Opacity" (Variables|Default|GetOpacity) :!class /Script/Engine.MaterialInstanceDynamic))))

(event Custom|Visible
  (bind _alpha (Timeline|TimelineVisible Play)
    (:Update
      (Variables|Default|SetOpacity (Math|Float|Lerp 0.0 1.0 _alpha))
      (Rendering|Material|SetScalarParameterValue (Variables|Default|GetMaterial) "Opacity" (Variables|Default|GetOpacity) :!class /Script/Engine.MaterialInstanceDynamic))))

(event EventBeginPlay)

(event Collision|EventActorBeginOverlap
  (params (OtherActor :type Actor%20Object%20Reference)))

(event EventTick
  (params (DeltaSeconds :type Float%20%28single-precision%29)))

(fn ConstructionScript
  (bind _returnvalue (Rendering|Material|CreateDynamicMaterialInstance (Variables|Default|GetStaticMesh) 0 "/Game/Asset/MI_Blackout.MI_Blackout" "None" :!class /Script/Engine.PrimitiveComponent))
  (Rendering|Material|SetScalarParameterValue _returnvalue "Opacity" (Variables|Default|GetOpacity) :!class /Script/Engine.MaterialInstanceDynamic)
  (Variables|Default|SetMaterial _returnvalue))