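; Capsule prop actor that randomly shows or omits a posed, spotlit figure.
; On BeginPlay a coin flip either plays one random non-looping female pose animation on the skeletal mesh, or destroys that mesh, both spotlights and a secondary static mesh.
; The pose plays in single-node animation mode, and the construction script is empty.
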(event EventBeginPlay
  (bind _skeletalmesh (Variables|Default|GetSkeletalMesh))
  (if (Math|Random|RandomBool)
    (Components|Animation|SetAnimationMode _skeletalmesh "AnimationSingleNode" true)
    (Components|Animation|PlayAnimation _skeletalmesh (.OutItem (Utilities|Array|Random (Utilities|Array|MakeArray "/Game/Asset/CharAsset/Female_Dance_Pose.Female_Dance_Pose" "/Game/Asset/CharAsset/Female_Dance_Pose__1_.Female_Dance_Pose__1_" "/Game/Asset/CharAsset/Female_Dynamic_Pose_Anim.Female_Dynamic_Pose_Anim" "/Game/Asset/CharAsset/Female_Standing_Pose.Female_Standing_Pose" "/Game/Asset/CharAsset/Female_Standing_Pose__1_.Female_Standing_Pose__1_"))) false)
    (else
      (Components|DestroyComponent (Variables|Default|GetSpotLight1)))))

(fn ConstructionScript)