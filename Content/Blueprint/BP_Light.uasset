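; BP_Light is a spot light actor whose intensity animates in repeated bursts at random intervals, with its construction script setting it to Max.
; After BeginPlay and a random delay of a few seconds, the Effect event plays a timeline that drives intensity between MIn and Max.
; When the timeline finishes, another random delay calls Effect again, looping indefinitely without Tick.
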(event Custom|Effect
  (bind _alpha (Timeline|EffectTimeline PlayFromStart)
    (:Update
      (Rendering|Components|Light|SetIntensity (Variables|Default|GetSpotLight) (Math|Float|Lerp (Variables|Default|GetMIn) (Variables|Default|GetMax) _alpha)))
    (:Finished
      (Utilities|FlowControl|Delay (Math|Random|RandomFloatinRange 1.0 5.0))
      (CallFunction|Effect))))

(event EventBeginPlay
  (Utilities|FlowControl|Delay (Math|Random|RandomFloatinRange 1.0 5.0))
  (CallFunction|Effect))

(event Collision|EventActorBeginOverlap
  (params (OtherActor :type Actor%20Object%20Reference)))

(event EventTick
  (params (DeltaSeconds :type Float%20%28single-precision%29)))

(fn ConstructionScript
  (Rendering|Components|Light|SetIntensity (Variables|Default|GetSpotLight) (Variables|Default|GetMax)))