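; AI controller for Enemy1 that caches the possessed BP_Enemy1, runs its behavior tree and tracks a sighted player.
; On perception updates, CanSense accepts only BP_Player actors with a successful sight stimulus and writes them to the TargetActor blackboard key.
; When perception forgets a target, it prints a debug string and CheckForget attempts to clear TargetActor if it matches that actor.
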(event OnPerceptionUpdated(AIPerception)
  (params (UpdatedActors :type Array%20of%20Actor%20Object%20References))
  (for _array_element UpdatedActors
    (Utilities|FlowControl|Sequence
      (:then_0
        (bind (_sense _stimulus) (CallFunction|CanSense _array_element "/Script/AIModule.AISense_Sight"))
        (if _sense
          (AI|Components|Blackboard|SetValueasObject (Variables|Default|GetBlackboard) (Utilities|Name|MakeLiteralName "TargetActor") _array_element))))))

(event OnTargetPerceptionForgotten(AIPerception)
  (params (Actor :type Actor%20Object%20Reference))
  (Development|PrintString "Hello")
  (CallFunction|CheckForget Actor))

(event EventBeginPlay)

(event EventTick
  (params (DeltaSeconds :type Float%20%28single-precision%29)))

(event EventPossess
  (params (PossessedPawn :type Pawn%20Object%20Reference))
  (bind _asbp_enemy_1 (Utilities|Casting|CastToBP_Enemy1 PossessedPawn))
  (Variables|Default|SetEnemy _asbp_enemy_1)
  (AI|RunBehaviorTree "/Game/Blueprint/Enemy/AI/BT_Enemy1.BT_Enemy1"))

(fn ConstructionScript)

(fn CanSense
  (params (Actor :type Actor%20Object%20Reference) (StimulusClass :type Object%20Class%20Reference))
  (Utilities|Casting|CastToBP_Player Actor
    (:then
      (bind _info (Class|AIPerceptionComponent|GetActorsPerception (Variables|Default|GetAIPerception) Actor))
      (for _array_element (.LastSensedStimuli (Utilities|Struct|BreakActorPerceptionBlueprintInfo _info))
        (bind _returnvalue (Class|AIPerceptionSystem|GetSenseClassforStimulus _array_element))
        (if (and (== _returnvalue StimulusClass) (.bSuccessfullySensed (Utilities|Struct|BreakAIStimulus _array_element)))
          (return true _array_element)))
      (return false ""))
    (:CastFailed
      (return false ""))))

(fn CheckForget
  (params (Actor :type Actor%20Object%20Reference))
  (bind _returnvalue (Class|AIPerceptionComponent|GetActorsPerception (Variables|Default|GetAIPerception)))
  (if (and _returnvalue (== Actor (AI|Components|Blackboard|GetValueasObject (Variables|Default|GetBlackboard) (Utilities|Name|MakeLiteralName "TargetActor"))))
    (AI|Components|Blackboard|SetValueasObject (Variables|Default|GetBlackboard) (Utilities|Name|MakeLiteralName "TargetActor") 0)))