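; Enemy character that can fade between visible and nearly invisible, with game logic delegated to its AIC_Enemy1 controller.
; Construction creates opaque and transparent dynamic materials; events swap between them or fade the transparent one's opacity through a reversible timeline.
; WrapMovement sets a motion-warp target for a jump attack, facing the target location.
; Damage is forwarded to the controller's Hit, and Die disables capsule collision.
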(event Custom|BecomeInvisible
  (if (not (== (Variables|Default|GetcurrentOpacity) 0.1))
    (bind _alpha (Timeline|Timeline Play)
      (:Update
        (Rendering|Material|SetScalarParameterValue (Variables|Default|GetMaterialTransparent) "Opacity" (Math|Float|Lerp 1.0 0.01 _alpha) :!class /Script/Engine.MaterialInstanceDynamic)
        (Variables|Default|SetcurrentOpacity (Math|Float|Lerp 1.0 0.01 _alpha))))))

(event Custom|BecomeVisible
  (if (not (== (Variables|Default|GetcurrentOpacity) 1.0))
    (bind _alpha (Timeline|Timeline Reverse)
      (:Update
        (Rendering|Material|SetScalarParameterValue (Variables|Default|GetMaterialTransparent) "Opacity" (Math|Float|Lerp 1.0 0.01 _alpha) :!class /Script/Engine.MaterialInstanceDynamic)
        (Variables|Default|SetcurrentOpacity (Math|Float|Lerp 1.0 0.01 _alpha))))))

(event Custom|WrapMovement
  (params (TargetLocation :type Vector))
  (Class|MotionWarpingComponent|AddorUpdateWarpTarget (Variables|Default|GetMotionWarping) (Utilities|Struct|MakeMotionWarpingTarget "JumpAttack" TargetLocation (Math|Rotator|FindLookatRotation (Transformation|GetActorLocation) TargetLocation) 0 "None" false "0.000000,0.000000,0.000000" "0.000000,0.000000,0.000000")))

(event Custom|Die
  (Collision|SetCollisionEnabled (Variables|Collision|GetCapsuleComponent) "NoCollision"))

(event EventBeginPlay
  (bind _asaic_enemy_1 (Utilities|Casting|CastToAIC_Enemy1 (Pawn|GetController)))
  (Variables|Default|SetAIController _asaic_enemy_1))

(event Collision|EventActorBeginOverlap
  (params (OtherActor :type Actor%20Object%20Reference)))

(event EventTick
  (params (DeltaSeconds :type Float%20%28single-precision%29)))

(event Game|Damage|EventAnyDamage
  (params (Damage :type Float%20%28single-precision%29) (DamageType :type Damage%20Type%20Object%20Reference) (InstigatedBy :type Controller%20Object%20Reference) (DamageCauser :type Actor%20Object%20Reference))
  (Default|Hit (Variables|Default|GetAIController) Damage))

(event EventGoVisible
  (Rendering|Material|SetMaterial (Variables|Character|GetMesh) 0 (Variables|Default|GetMaterialVisible)))

(event EventGoTransparent
  (Rendering|Material|SetMaterial (Variables|Character|GetMesh) 0 (Variables|Default|GetMaterialTransparent)))

(fn ConstructionScript
  (Utilities|FlowControl|Sequence
    (:then_0
      (bind _returnvalue (Rendering|Material|CreateDynamicMaterialInstance (Variables|Character|GetMesh) 0 "/Game/Asset/Enemy1/M_VIsibleEnemy1.M_VIsibleEnemy1" "None" :!class /Script/Engine.PrimitiveComponent))
      (Variables|Default|SetMaterialVisible _returnvalue))
    (:then_1
      (bind _returnvalue_2 (Rendering|Material|CreateDynamicMaterialInstance (Variables|Character|GetMesh) 0 "/Game/Asset/Enemy1/MI_Enemy1.MI_Enemy1" "None" :!class /Script/Engine.PrimitiveComponent))
      (bind _output_get (Variables|Default|SetMaterialTransparent _returnvalue_2))
      (Rendering|Material|SetScalarParameterValue (Variables|Default|GetMaterialTransparent) "Opacity" 0.01 :!class /Script/Engine.MaterialInstanceDynamic))))