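; BP_Chest is a one-shot loot chest that opens and drops random items when the player enters its trigger box.
; On overlap with BP_Player it destroys the trigger, plays the OpenCase timeline to rotate the CloseCase component, and spawns a few random picks from ItemList.
; Items spawn at the chest's location, each given a random TargetLocation within the central half-extent region of the DropPosition box.
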(event OnComponentBeginOverlap(Box)
  (params (OverlappedComponent :type Primitive%20Component%20Object%20Reference) (OtherActor :type Actor%20Object%20Reference) (OtherComp :type Primitive%20Component%20Object%20Reference) (OtherBodyIndex :type Integer) (bFromSweep :type Boolean) (SweepResult :type Hit%20Result%20Structure%20%28by%20ref%29))
  (bind _dropposition (Variables|Default|GetDropPosition))
  (bind _returnvalue (Transformation|GetWorldLocation _dropposition))
  (bind _boxextent (Variables|/Script/Engine.BoxComponent|GetBoxExtent _dropposition))
  (bind _returnvalue_2 (/ _boxextent 2.0))
  (Utilities|Casting|CastToBP_Player OtherActor)
  (Components|DestroyComponent (Variables|Default|GetBox))
  (Utilities|FlowControl|Sequence
    (:then_0
      (bind _alpha (Timeline|OpenCase Play)
        (:Update
          (Transformation|SetRelativeRotation (Variables|Default|GetCloseCase) (Math|Rotator|MakeRotator (Math|Float|Lerp 105.0 0.0 _alpha) 0.0 0.0) false false))))
    (:then_1
      (bind _output_get (Variables|Default|SetRandomObjectNumber (Math|Random|RandomIntegerinRange 1 3)))
      (for _index (range 1 _output_get)
        (Game|SpawnActorfromClass (.OutItem (Utilities|Array|Random (Variables|Default|GetItemList))) (Math|Conversions|ToTransform(Vector) (Transformation|GetActorLocation)) "AlwaysSpawn" "MultiplyWithRoot" 0 (Class|KismetMathLibrary|RandomPointinBoundingBoxBox (Math|Box|MakeBox (- _returnvalue _returnvalue_2) (+ _returnvalue _returnvalue_2))) 0)))))

(event EventBeginPlay)

(event Collision|EventActorBeginOverlap
  (params (OtherActor :type Actor%20Object%20Reference)))

(event EventTick
  (params (DeltaSeconds :type Float%20%28single-precision%29)))

(fn ConstructionScript)