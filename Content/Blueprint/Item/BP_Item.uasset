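; Pickup item that spins, applies an effect to BP_Player on box overlap, plays a pickup sound and destroys itself.
; After a short delay, the SpawnTrack timeline moves it from its spawn point to TargetLocation, adding a math-expression-driven height offset.
; The Effect event is empty here, leaving a hook for specific item behavior.
; The construction script applies IconTexture to the Plane through a dynamic material instance.
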(event OnComponentBeginOverlap(Box)
  (params (OverlappedComponent :type Primitive%20Component%20Object%20Reference) (OtherActor :type Actor%20Object%20Reference) (OtherComp :type Primitive%20Component%20Object%20Reference) (OtherBodyIndex :type Integer) (bFromSweep :type Boolean) (SweepResult :type Hit%20Result%20Structure%20%28by%20ref%29))
  (bind _asbp_player (Utilities|Casting|CastToBP_Player OtherActor))
  (CallFunction|Effect _asbp_player)
  (Audio|PlaySoundatLocation "/Game/Asset/Audio/C_TakeObjects.C_TakeObjects" (Transformation|GetActorLocation) "0, 0, 0" 1.0 1.0 0.0 0 0 0 0)
  (Actor|DestroyActor))

(event Custom|Effect
  (params (Player :type BP%20Player%20Object%20Reference)))

(event EventBeginPlay
  (Utilities|FlowControl|Delay 0.5)
  (Variables|Default|SetInitLocation (Transformation|GetActorLocation))
  (bind _alpha (Timeline|SpawnTrack Play)
    (:Update
      (Transformation|SetActorLocation (+ (Math|Vector|Lerp(Vector) (Variables|Default|GetInitLocation) (Variables|Default|GetTargetLocation) _alpha) (Math|Vector|MakeVector 0.0 0.0 (Math|Float|Lerp 0.0 1e+02 (|(((3-7)*(pow((x-0.500000),2)))+1) _alpha)))) false false))))

(event Collision|EventActorBeginOverlap
  (params (OtherActor :type Actor%20Object%20Reference)))

(event EventTick
  (params (DeltaSeconds :type Float%20%28single-precision%29))
  (Class|Actor|AddActorWorldRotation "0.000000,1.000000,0.000000"))

(fn ConstructionScript
  (bind _returnvalue (Rendering|Material|CreateDynamicMaterialInstance (Variables|Default|GetPlane) 0 0 "None" :!class /Script/Engine.PrimitiveComponent))
  (Rendering|Material|SetTextureParameterValue _returnvalue "IconTexture" (Variables|Default|GetIconTexture)))