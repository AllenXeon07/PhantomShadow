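; BP_Lift is a lift objective whose sliding doors open for the player and which ends the level through the game mode.
; Overlapping the Box trigger plays the DoorOpen timeline, moving two door cubes apart in mirrored motion, and leaving reverses it.
; A Lock flag blocks both opening and closing.
; A BP_Player entering the second trigger, Box1, calls Finish on GM_GamePlay, independent of the lock.
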(event OnComponentBeginOverlap(Box)
  (params (OverlappedComponent :type Primitive%20Component%20Object%20Reference) (OtherActor :type Actor%20Object%20Reference) (OtherComp :type Primitive%20Component%20Object%20Reference) (OtherBodyIndex :type Integer) (bFromSweep :type Boolean) (SweepResult :type Hit%20Result%20Structure%20%28by%20ref%29))
  (Utilities|Casting|CastToBP_Player OtherActor)
  (CallFunction|OpentheLift))

(event OnComponentEndOverlap(Box)
  (params (OverlappedComponent :type Primitive%20Component%20Object%20Reference) (OtherActor :type Actor%20Object%20Reference) (OtherComp :type Primitive%20Component%20Object%20Reference) (OtherBodyIndex :type Integer))
  (Utilities|Casting|CastToBP_Player OtherActor)
  (CallFunction|ClosetheLift))

(event OnComponentBeginOverlap(Box1)
  (params (OverlappedComponent :type Primitive%20Component%20Object%20Reference) (OtherActor :type Actor%20Object%20Reference) (OtherComp :type Primitive%20Component%20Object%20Reference) (OtherBodyIndex :type Integer) (bFromSweep :type Boolean) (SweepResult :type Hit%20Result%20Structure%20%28by%20ref%29))
  (Utilities|Casting|CastToBP_Player OtherActor)
  (Default|Finish (.AsGM%20Game%20Play (Utilities|Casting|CastToGM_GamePlay (Game|GetGameMode)))))

(event Custom|OpenTheLift
  (if (not (Variables|Default|GetLock?))
    (bind _alpha (Timeline|DoorOpen Play)
      (:Update
        (Transformation|SetRelativeLocation (Variables|Default|GetCube) (Math|Vector|MakeVector -257.0 (Math|Float|Lerp 138.0 386.0 _alpha) 5e+01) false false)
        (Transformation|SetRelativeLocation (Variables|Default|GetCube1) (Math|Vector|MakeVector -257.0 (* (Math|Float|Lerp 138.0 386.0 _alpha) -1.0) 5e+01) false false)))))

(event Custom|CloseTheLift
  (if (not (Variables|Default|GetLock?))
    (bind _alpha (Timeline|DoorOpen Reverse)
      (:Update
        (Transformation|SetRelativeLocation (Variables|Default|GetCube) (Math|Vector|MakeVector -257.0 (Math|Float|Lerp 138.0 386.0 _alpha) 5e+01) false false)
        (Transformation|SetRelativeLocation (Variables|Default|GetCube1) (Math|Vector|MakeVector -257.0 (* (Math|Float|Lerp 138.0 386.0 _alpha) -1.0) 5e+01) false false)))))

(event EventBeginPlay)

(event Collision|EventActorBeginOverlap
  (params (OtherActor :type Actor%20Object%20Reference)))

(event EventTick
  (params (DeltaSeconds :type Float%20%28single-precision%29)))

(fn ConstructionScript)