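; BP_LockDoor is a door Blueprint that refuses to open while its Lock flag is set.
; On BeginPlay it creates a "need a key" notification, assigns it to its Widget component and hides that component.
; OpentheDoor shows the notification for two seconds when locked, and otherwise defers to the parent class's door-opening logic.
; Nothing in this Blueprint changes Lock.
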(event EventBeginPlay
  (|CallParentFunction)
  (bind _returnvalue (UserInterface|CreateWidget "/Game/Blueprint/Objectives/WB_Notification.WB_Notification_C" 0 "NEED A KEY !!!"))
  (UserInterface|SetWidget (Variables|Default|GetWidget) _returnvalue)
  (Variables|Default|SetNotifWB _returnvalue)
  (Development|SetHiddeninGame (Variables|Default|GetWidget) true false))

(event Collision|EventActorBeginOverlap
  (params (OtherActor :type Actor%20Object%20Reference))
  (|CallParentFunction OtherActor) ; This node is disabled and will not be called.\nDrag off pins to build functionality.
)

(event EventTick
  (params (DeltaSeconds :type Float%20%28single-precision%29))
  (|CallParentFunction DeltaSeconds) ; This node is disabled and will not be called.\nDrag off pins to build functionality.
)

(event EventOpentheDoor
  (if (Variables|Default|Getlock?)
    (Development|SetHiddeninGame (Variables|Default|GetWidget) false false)
    (Utilities|FlowControl|Delay 2.0)
    (Development|SetHiddeninGame (Variables|Default|GetWidget) true false)
    (else
      (|CallParentFunction))))

(fn ConstructionScript
  (|CallParentFunction))