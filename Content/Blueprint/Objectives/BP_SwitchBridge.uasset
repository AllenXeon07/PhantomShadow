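; BP_SwitchBridge is a one-shot switch that opens access on a referenced bridge when the player touches it.
; When BP_Player overlaps the trigger Box, it destroys the Box to prevent retriggering and immediately calls OpenAccess on Bridge.
; A SwitchRotate timeline then swings the switch mesh's pitch from one side to the other and plays a sound at the actor's location when finished.
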(event OnComponentBeginOverlap(Box)
  (params (OverlappedComponent :type Primitive%20Component%20Object%20Reference) (OtherActor :type Actor%20Object%20Reference) (OtherComp :type Primitive%20Component%20Object%20Reference) (OtherBodyIndex :type Integer) (bFromSweep :type Boolean) (SweepResult :type Hit%20Result%20Structure%20%28by%20ref%29))
  (Utilities|Casting|CastToBP_Player OtherActor)
  (Components|DestroyComponent (Variables|Default|GetBox))
  (Default|OpenAccess (Variables|Default|GetBridge))
  (bind _alpha (Timeline|SwitchRotate PlayFromStart)
    (:Update
      (Transformation|SetRelativeRotation (Variables|Default|GetMerge_BF181D9B) (Math|Rotator|MakeRotator 0.0 (Math|Float|Lerp -3e+01 3e+01 _alpha) 0.0) false false))
    (:Finished
      (Audio|PlaySoundatLocation "/Game/Victorian_House/Audio/Cues/Cue_Light.Cue_Light" (Transformation|GetActorLocation) "0, 0, 0" 1.0 1.0 0.0 0 0 0 0))))

(event EventBeginPlay)

(event Collision|EventActorBeginOverlap
  (params (OtherActor :type Actor%20Object%20Reference)))

(event EventTick
  (params (DeltaSeconds :type Float%20%28single-precision%29)))

(fn ConstructionScript)