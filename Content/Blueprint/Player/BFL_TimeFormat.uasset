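; Blueprint function library that formats an integer time value as clock-style text, by its name and path for player-related timers.
; TimerFormat splits the value by 60 into quotient and remainder and joins them with a colon, giving a minutes:seconds string.
; DetailFormat supplies each part, prepending a zero when the number is below ten.
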(fn DetailFormat
  (params (Number :type Integer))
  (bind _returnvalue (Utilities|String|ToString(Integer) Number))
  (return (select (< Number 10) (Utilities|String|Append "0" _returnvalue) _returnvalue)))

(fn TimerFormat
  (params (Timer :type Integer))
  (return (Utilities|String|Append (CallFunction|DetailFormat (/ Timer 60)) ":" (CallFunction|DetailFormat (Math|Integer|%(Integer) Timer 60)))))