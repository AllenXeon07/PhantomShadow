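; BPC_BatteryReduce is an actor component that drains the player's battery and stops X-ray when it runs out.
; On BeginPlay it caches its owner as BP_Player and slows its tick interval to a tenth of a second.
; Each tick decrements Battery by a fixed step without delta-time scaling and passes it to SetBatteryPercentage, or calls StopXRay once the charge is empty.
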(event EventBeginPlay
  (Class|ActorComponent|SetComponentTickInterval 0.1)
  (bind _asbp_player (Utilities|Casting|CastToBP_Player (Components|GetOwner)))
  (Variables|Default|SetOwner _asbp_player))

(event EventTick
  (params (DeltaSeconds :type Float%20%28single-precision%29))
  (bind _owner (Variables|Default|GetOwner))
  (bind _owner_2 (Variables|Default|GetOwner))
  (Utilities|IsValid _owner
    (:Is%20Valid
      (if (> (Variables|/Game/Blueprint/Player/BP_Player.BP_Player_C|GetBattery _owner) 0.0)
        (bind _result (Math|Float|DecrementFloat (Variables|/Game/Blueprint/Player/BP_Player.BP_Player_C|GetBattery _owner_2))
          (:%20%20
            (Default|SetBatteryPercentage _owner_2 _result)))
        (else
          (Default|StopXRay _owner_2))))))