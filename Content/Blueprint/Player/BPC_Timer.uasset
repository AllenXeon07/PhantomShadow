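; Timer component for the GM_GamePlay game mode that counts elapsed time and shows it on the HUD.
; BeginPlay sets a one-second tick interval, resets the count and caches the owning game mode.
; Each tick increments the count and passes it to the HUD's SetTimer.
; Stop sets the tick interval to zero, which makes ticks run every frame instead of disabling them.
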(event Custom|Stop
  (Class|ActorComponent|SetComponentTickInterval 0.0))

(event EventBeginPlay
  (Class|ActorComponent|SetComponentTickInterval 1.0)
  (Variables|Default|SetTime 0)
  (bind _asgm_game_play (Utilities|Casting|CastToGM_GamePlay (Components|GetOwner)))
  (Variables|Default|SetGM _asgm_game_play))

(event EventTick
  (params (DeltaSeconds :type Float%20%28single-precision%29))
  (bind _result (Math|Integer|IncrementInt (Variables|Default|GetTime))
    (:%20%20
      (Default|SetTimer (Variables|/Game/Blueprint/Player/GM_GamePlay.GM_GamePlay_C|GetHUD (Variables|Default|GetGM)) _result))))