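; GI_GamePlay, a game instance by its prefix, holds high scores per level and persists them through a save game.
; SaveGame creates an SG_Game object if none is valid, copies HighScore into it and writes it to a fixed slot.
; LoadGame restores HighScore from that slot, or falls back to SaveGame when the slot is missing or the cast fails.
; GetHighscore returns the HighScore entry for the current Level.
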(event Custom|SaveGame
  (Utilities|IsValid (Variables|Default|GetSave)
    (:Is%20Valid
      _)
    (:Is%20Not%20Valid
      (bind _returnvalue (SaveGame|CreateSaveGameObject "/Game/Blueprint/Player/SG_Game.SG_Game_C"))
      (Variables|Default|SetSave _returnvalue)))
  (Variables|/Game/Blueprint/Player/SG_Game.SG_Game_C|SetHighscore (Variables|Default|GetSave) (Variables|Default|GetHighScore))
  (SaveGame|SaveGametoSlot (Variables|Default|GetSave) "SaveGame"))

(event Custom|LoadGame
  (bind _returnvalue (SaveGame|DoesSaveGameExist "SaveGame"))
  (if _returnvalue
    (bind _returnvalue_2 (SaveGame|LoadGamefromSlot "SaveGame"))
    (bind _assg_game (Utilities|Casting|CastToSG_Game _returnvalue_2)
      (:then
        (bind _output_get (Variables|Default|SetSave _assg_game))
        (Variables|Default|SetHighScore (Variables|/Game/Blueprint/Player/SG_Game.SG_Game_C|GetHighscore _output_get)))
      (:CastFailed
        (CallFunction|SaveGame :!label _label)))
    (else
      (goto _label))))

(fn GetHighscore
  (return (Utilities|Array|Get(acopy) (Variables|Default|GetHighScore) (Variables|Default|GetLevel))))