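; GM_GamePlay is the gameplay game mode that sets up the player and HUD when play begins.
; On BeginPlay it spawns BP_Player at the location of a PlayerStart, possesses it with player controller 0 and stores it.
; It then creates WB_HUD, adds it to the viewport, hands it to the player and calls the player's SetupPlayer.
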(event EventBeginPlay
  (bind _returnvalue (Actor|GetActorOfClass "/Script/Engine.PlayerStart"))
  (bind _returnvalue_2 (Game|SpawnActorfromClass "/Game/Blueprint/Player/BP_Player.BP_Player_C" (Math|Conversions|ToTransform(Vector) (Transformation|GetActorLocation _returnvalue)) "Undefined" "MultiplyWithRoot" 0 0))
  (Pawn|Possess (Game|GetPlayerController 0) _returnvalue_2)
  (Variables|Default|SetPlayer _returnvalue_2)
  ;[1 1 1] Create Widget
  (bind _returnvalue_3 (UserInterface|CreateWidget "/Game/Blueprint/Player/WB_HUD.WB_HUD_C"))
  (Variables|Default|SetHUD _returnvalue_3)
  (UserInterface|Viewport|AddtoViewport _returnvalue_3 0)
  (Variables|/Game/Blueprint/Player/BP_Player.BP_Player_C|SetHUD (Variables|Default|GetPlayer) (Variables|Default|GetHUD))
  (Default|SetupPlayer (Variables|Default|GetPlayer)))

(event EventTick
  (params (DeltaSeconds :type Float%20%28single-precision%29)))

(fn ConstructionScript)