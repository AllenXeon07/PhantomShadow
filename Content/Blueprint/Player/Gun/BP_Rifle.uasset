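; BP_Rifle is a pickup rifle that attaches to the player's Weapon socket on overlap and registers as their gun.
; StartShoot and Reload play player montages, using their durations to time shots and magazine refills, and an empty magazine triggers a reload.
; A separate Shoot event, not called within this graph, damages BP_Enemy1 pawns along a multi line trace and moves a detached Niagara trail along that line.
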(event OnComponentBeginOverlap(Box)
  (params (OverlappedComponent :type Primitive%20Component%20Object%20Reference) (OtherActor :type Actor%20Object%20Reference) (OtherComp :type Primitive%20Component%20Object%20Reference) (OtherBodyIndex :type Integer) (bFromSweep :type Boolean) (SweepResult :type Hit%20Result%20Structure%20%28by%20ref%29))
  (bind _asbp_player (Utilities|Casting|CastToBP_Player OtherActor))
  (Variables|Default|SetPlayer _asbp_player)
  (Collision|SetCollisionEnabled (Variables|Default|GetBox) "NoCollision")
  (Transformation|AttachComponentToComponent self (Variables|/Script/Engine.Character|GetMesh _asbp_player) "Weapon" "SnapToTarget" "SnapToTarget" "KeepRelative" true)
  (Variables|/Game/Blueprint/Player/BP_Player.BP_Player_C|SetGun _asbp_player self))

(event Custom|StartShoot
  (if (not (Variables|Default|GetReload?))
    (if (<= (Variables|Default|GetMagazineAmmo) 0)
      (CallFunction|Reload)
      (elif (not (Variables|Default|GetShooting?))
        (Variables|Default|SetShooting? true)
        (bind _returnvalue (Animation|PlayAnimMontage (Variables|Default|GetPlayer) "/Game/Asset/Player/AM_Shoot.AM_Shoot" 1.0 "None"))
        (Utilities|FlowControl|Delay (* _returnvalue 0.3))
        (Variables|Default|SetMagazineAmmo (- (Variables|Default|GetMagazineAmmo) 1))
        (CallFunction|StopShoot)))))

(event Custom|StopShoot
  (Variables|Default|SetShooting? false))

(event Custom|Shoot
  (bind _attackradius (Variables|Default|GetAttackRadius))
  (bind _arrow (Variables|Default|GetArrow))
  (bind _arrow_2 (Variables|Default|GetArrow))
  (bind _ns_bullettrail (Variables|Default|GetNS_BulletTrail))
  (bind _returnvalue (Transformation|GetWorldLocation _arrow))
  (bind _returnvalue_2 (Math|Vector|GetForwardVector _arrow))
  (bind _returnvalue_3 (Transformation|GetWorldLocation _arrow_2))
  (bind _returnvalue_4 (* _returnvalue_2 _attackradius))
  (bind _returnvalue_5 (+ _returnvalue _returnvalue_4))
  (bind _returnvalue_6 (Math|Rotator|FindLookatRotation _returnvalue _returnvalue_5))
  (Components|Activation|Deactivate (Variables|Default|GetNS_BulletTrail))
  (Utilities|FlowControl|Sequence
    (:then_0
      (bind _outhits (Class|KismetSystemLibrary|LineTraceMultiforObjects _returnvalue_3 (+ _returnvalue_3 (* (Math|Vector|GetForwardVector _arrow_2) (Variables|Default|GetAttackRadius))) (Utilities|Array|MakeArray "ObjectTypeQuery3") false 0 "None" true))
      (for _array_element _outhits
        (bind _asbp_enemy_1 (Utilities|Casting|CastToBP_Enemy1 (.HitActor (Collision|BreakHitResult _array_element))))
        (Game|Damage|ApplyDamage _asbp_enemy_1 1e+01 0 (Variables|Default|GetPlayer))))
    (:then_1
      (Transformation|DetachFromComponent _ns_bullettrail "KeepWorld" "KeepWorld" "KeepWorld" true)
      (Transformation|SetWorldLocation _ns_bullettrail (Transformation|GetWorldLocation (Variables|Default|GetArrow)) false true)
      (Transformation|SetWorldRotation _ns_bullettrail _returnvalue_6 false false)
      (Components|Activation|Activate _ns_bullettrail true)
      (Components|MoveComponentTo (Variables|Default|GetNS_BulletTrail) _returnvalue_5 _returnvalue_6 false false 0.5 true)
      (Components|Activation|Deactivate (Variables|Default|GetNS_BulletTrail)))))

(event Custom|Reload
  (if (not (Variables|Default|GetReload?))
    (Development|PrintString "Hello")
    (Variables|Default|SetReload? true)
    (bind _returnvalue (Animation|PlayAnimMontage (Variables|Default|GetPlayer) "/Game/Asset/Player/AM_Reload.AM_Reload" 1.0 "None"))
    (Utilities|FlowControl|Delay _returnvalue)
    (Variables|Default|SetMagazineAmmo (Variables|Default|GetMaxMagazineAmmo))
    (Variables|Default|SetReload? false)))

(event EventBeginPlay
  (Variables|Default|SetMagazineAmmo (Variables|Default|GetMaxMagazineAmmo)))

(event Collision|EventActorBeginOverlap
  (params (OtherActor :type Actor%20Object%20Reference)))

(event EventTick
  (params (DeltaSeconds :type Float%20%28single-precision%29)))

(fn ConstructionScript)